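; PoliceCar_BP is a police car that drives by applying forces and rotations to a physics-simulated Plane component.
; Accelerate and Reverse push along the forward vector, while Brake applies force along the velocity direction.
; TurnRight sets a speed-scaled target yaw, which Tick interpolates toward.
; Tick also applies friction opposing the previous frame's velocity, strengthened as that velocity's yaw diverges from the car's heading.
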(event Custom|Reverse
  (params (Amount :type Float%20%28single-precision%29))
  (Physics|AddForce (Variables|Default|GetPlane) (* (Math|Vector|GetForwardVector (Variables|Default|GetPlane)) (* Amount (Variables|Parameters|GetAcceleration%20Amount))) "None" true))

(event Custom|Brake
  (params (Amount :type Float%20%28single-precision%29))
  (bind _returnvalue (Physics|GetPhysicsLinearVelocity (Variables|Default|GetPlane) "None"))
  (if (> (Math|Vector|VectorLength _returnvalue) 0.0)
    (Physics|AddForce (Variables|Default|GetPlane) (* (Math|Vector|Normalize _returnvalue) (* Amount (Variables|Parameters|GetBrake%20Amount))) "None" true)))

(event Custom|Accelerate
  (params (Amount :type Float%20%28single-precision%29))
  (Physics|AddForce (Variables|Default|GetPlane) (* (Math|Vector|GetForwardVector (Variables|Default|GetPlane)) (* Amount (Variables|Parameters|GetAcceleration%20Amount))) "None" true))

(event Custom|Turn%20Right
  (params (Amount :type Float%20%28single-precision%29))
  (bind _plane (Variables|Default|GetPlane))
  (bind _returnvalue (Transformation|GetWorldRotation _plane))
  (Variables|Turning|SetTurn%20Direction Amount)
  (bind _returnvalue_2 (Physics|GetPhysicsLinearVelocity (Variables|Default|GetPlane) "None"))
  (bind _output_get (Variables|Turning|SetTurnAngle (* Amount (* (Variables|Parameters|GetMaxTurn) (Math|Float|MapRangeClamped (Math|Float|Absolute(Float) (Math|Vector|VectorLength _returnvalue_2)) 0.0 1e+03 0.0 1.0)))))
  (Variables|Turning|SetDesired%20Angle (+ _output_get (.yaw _returnvalue)))
  (Variables|Turning|SetCurrent%20Angle (.yaw _returnvalue))
  (Variables|Turning|SetCurr%20Turn%20Time 0.0))

(event EventTick
  (params (DeltaSeconds :type Float%20%28single-precision%29))
  (bind _plane (Variables|Default|GetPlane))
  (bind _returnvalue (Transformation|GetWorldRotation _plane))
  (Utilities|FlowControl|Sequence
    (:then_0
      ;[1 1 1] Turning
      (if (!= (Variables|Turning|GetCurrent%20Angle) (Variables|Turning|GetDesired%20Angle))
        (Variables|Turning|SetCurr%20Turn%20Time (+ (Variables|Turning|GetCurr%20Turn%20Time) DeltaSeconds))
        (Transformation|SetWorldRotation (Variables|Default|GetPlane) (Math|Rotator|MakeRotator (.roll _returnvalue) (.pitch _returnvalue) (Math|Float|Lerp (Variables|Turning|GetCurrent%20Angle) (Variables|Turning|GetDesired%20Angle) (Variables|Turning|GetCurr%20Turn%20Time))) false false)))
    (:then_1
      ;[1 1 1] Friction
      (Physics|AddForce (Variables|Default|GetPlane) (* (* (Variables|Default|GetPrev%20Friction) (+ (* (Math|Float|MapRangeClamped (Math|Float|Absolute(Float) (.yaw (CallFunction|GetRotationfromTwoVectors (Variables|Default|GetPrev%20Friction) (Math|Vector|GetForwardVector (Variables|Default|GetPlane))))) 0.0 9e+01 0.0 1.0) (Variables|Default|GetAngled%20Friction%20Multiplier)) 1.0)) -1.0) "None" true)
      (bind _returnvalue_2 (Physics|GetPhysicsLinearVelocity (Variables|Default|GetPlane) "None"))
      (Variables|Default|SetPrev%20Friction _returnvalue_2))))

(fn ConstructionScript
  (Variables|Turning|SetCurrent%20Angle (.yaw (Transformation|GetWorldRotation (Variables|Default|GetPlane)))))