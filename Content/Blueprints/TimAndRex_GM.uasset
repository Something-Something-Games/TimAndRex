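; TimAndRex_GM is the game mode Blueprint that spawns police cars into the level.
; On BeginPlay it gathers every PoliceSpawnPoint_BP actor and calls the SpawnPoliceCar event.
; SpawnPoliceCar places a PoliceCar_BP at a random spawn point's transform while the running car count is below the maximum, then increments the count.
; Only one spawn call runs at start; nothing here repeats it or decrements the count.
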(event Custom|Spawn%20Police%20Car
  (if (< (Variables|Default|GetPolice%20Cars) (Variables|Default|GetMax%20Police%20Cars))
    (Game|SpawnActorfromClass "/Game/Blueprints/PoliceCar_BP.PoliceCar_BP_C" (Transformation|GetWorldTransform (Variables|/Game/Blueprints/PoliceSpawnPoint_BP.PoliceSpawnPoint_BP_C|GetDefaultSceneRoot (.OutItem (Utilities|Array|Random (Variables|Default|GetPolice%20Spawn%20Points))))) "Undefined" 0 0)
    (Math|Integer|IncrementInt (Variables|Default|GetPolice%20Cars))))

(event EventBeginPlay
  (bind _outactors (Actor|GetAllActorsOfClass "/Game/Blueprints/PoliceSpawnPoint_BP.PoliceSpawnPoint_BP_C"))
  (Variables|Default|SetPolice%20Spawn%20Points _outactors)
  (CallFunction|SpawnPoliceCar))

(fn ConstructionScript)