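; EndController is a level-ending trigger actor that finishes the game when the TimAndRexCar_BP car enters its Box.
; On overlap it disables the car and starts a fast looping timer that nudges the Boat along negative world Y each tick of the timer.
; After a short delay it casts the game mode to TimAndRex_GM and calls EndGame.
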(event OnComponentBeginOverlap(Box)
  (params (OverlappedComponent :type Primitive%20Component%20Object%20Reference) (OtherActor :type Actor%20Object%20Reference) (OtherComp :type Primitive%20Component%20Object%20Reference) (OtherBodyIndex :type Integer) (bFromSweep :type Boolean) (SweepResult :type Hit%20Result%20Structure%20%28by%20ref%29))
  (bind _astim_and_rex_car_bp (Utilities|Casting|CastToTimAndRexCar_BP OtherActor))
  (bind _output_get (Variables|Default|SetTim%20And%20Rex%20Car _astim_and_rex_car_bp))
  (Default|DisableCar _output_get)
  (Utilities|Time|SetTimerbyEvent (delegate Custom|Move%20Boat) 0.01 true)
  (Utilities|FlowControl|Delay 3.0)
  (bind _astim_and_rex_gm (Utilities|Casting|CastToTimAndRex_GM (Game|GetGameMode)))
  (Default|EndGame _astim_and_rex_gm))

(event Custom|Move%20Boat
  (Transformation|AddActorWorldOffset (Variables|Default|GetBoat) "0,-5.000000, 0"))

(event EventBeginPlay)

(event Collision|EventActorBeginOverlap
  (params (OtherActor :type Actor%20Object%20Reference)))

(event EventTick
  (params (DeltaSeconds :type Float%20%28single-precision%29)))

(fn ConstructionScript)