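; Drivable physics car for Tim or Rex, moved by acceleration-change forces on its Plane component.
; Input events drive throttle, reverse, braking and speed-scaled yaw turning that Tick interpolates, with pitch and roll held at zero.
; A timeline serves as a speed-to-acceleration curve lookup, while Tick applies drag that rises above max speed.
; LoadCharacter pulls handling stats from a data table and tints the lights per character, with construction defaulting to Tim.
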(event Custom|Reverse
  (params (Amount :type Float%20%28single-precision%29))
  ;[1 1 1] Reverse
  (Physics|AddForce (Variables|Default|GetPlane) (* (Math|Vector|GetForwardVector (Variables|Default|GetPlane)) (* Amount (Variables|Parameters|GetReverse%20Amount))) "None" true))

(event Custom|Brake
  (params (Amount :type Float%20%28single-precision%29))
  ;[1 1 1] Braking
  (bind _returnvalue (Physics|GetPhysicsLinearVelocity (Variables|Default|GetPlane) "None"))
  (Physics|AddForce (Variables|Default|GetPlane) (* (* _returnvalue (+ (* (Math|Float|MapRangeClamped (Math|Float|Absolute(Float) (.yaw (CallFunction|GetRotationfromTwoVectors _returnvalue (Math|Vector|GetForwardVector (Variables|Default|GetPlane))))) 0.0 9e+01 0.0 1.0) (Variables|Parameters|GetBrake%20Amount)) 1.0)) Amount) "None" true))

(event Custom|Accelerate
  (params (Amount :type Float%20%28single-precision%29))
  ;[1 1 1] Acceleration
  (Variables|Default|SetAcceleration Amount)
  (bind _returnvalue (Physics|GetPhysicsLinearVelocity (Variables|Default|GetPlane) "None"))
  (CallFunction|LookupAcceleration (Math|Float|MapRangeClamped (Math|Vector|VectorLength _returnvalue) 0.0 5e+03 0.0 1.0)))

(event Custom|Lookup%20Acceleration
  (params (Lookup%20Value :type Float%20%28single-precision%29))
  ;[1 1 1] Acceleration
  (bind _acceleration (Timeline|Acceleration%20Lookup SetNewTime)
    (:Update
      (CallFunction|ReturnAccelerationLookup _acceleration))))

(event Custom|Turn%20Right
  (params (Amount :type Float%20%28single-precision%29))
  (bind _plane (Variables|Default|GetPlane))
  (bind _relativerotation (Variables|/Script/Engine.SceneComponent|GetRelativeRotation _plane))
  ;[1 1 1] Turning Input
  (Variables|Turning|SetTurn%20Direction Amount)
  (bind _returnvalue (Physics|GetPhysicsLinearVelocity (Variables|Default|GetPlane) "None"))
  (bind _output_get (Variables|Turning|SetTurnAngle (* Amount (* (Variables|Parameters|GetMaxTurn) (Math|Float|MapRangeClamped (Math|Float|Absolute(Float) (Math|Vector|VectorLength _returnvalue)) 0.0 1e+03 0.0 1.0)))))
  (Variables|Turning|SetDesired%20Angle (+ _output_get (.yaw _relativerotation)))
  (Variables|Turning|SetCurrent%20Angle (.yaw _relativerotation))
  (Variables|Turning|SetCurr%20Turn%20Time 0.0)
  (if (< (Variables|Turning|GetDesired%20Angle) 0.0)
    (Variables|Turning|SetDesired%20Angle (+ (Variables|Turning|GetDesired%20Angle) 3.6e+02))))

(event Custom|Return%20Acceleration%20Lookup
  (params (Acceleration :type Float%20%28single-precision%29))
  ;[1 1 1] Acceleration
  (Physics|AddForce (Variables|Default|GetPlane) (* (Math|Vector|GetForwardVector (Variables|Default|GetPlane)) (* (* Acceleration (Variables|Default|GetAcceleration)) (Variables|Parameters|GetAcceleration%20Amount))) "None" true))

(event EventTick
  (params (DeltaSeconds :type Float%20%28single-precision%29))
  (bind _plane (Variables|Default|GetPlane))
  (bind _plane_2 (Variables|Default|GetPlane))
  (bind _plane_3 (Variables|Default|GetPlane))
  (bind _relativerotation (Variables|/Script/Engine.SceneComponent|GetRelativeRotation _plane_2))
  (bind _relativerotation_2 (Variables|/Script/Engine.SceneComponent|GetRelativeRotation _plane_3))
  (Utilities|FlowControl|Sequence
    (:then_0
      ;[1 1 1] Turning
      (if (!= (Variables|Turning|GetCurrent%20Angle) (Variables|Turning|GetDesired%20Angle))
        (Variables|Turning|SetCurr%20Turn%20Time (+ (Variables|Turning|GetCurr%20Turn%20Time) DeltaSeconds))
        (Transformation|SetRelativeRotation (Variables|Default|GetPlane) (Math|Rotator|Lerp(Rotator) (Math|Rotator|MakeRotator (.roll _relativerotation_2) (.pitch _relativerotation_2) (Variables|Turning|GetCurrent%20Angle)) (Math|Rotator|MakeRotator (.roll _relativerotation) (.pitch _relativerotation) (Variables|Turning|GetDesired%20Angle)) (Variables|Turning|GetCurr%20Turn%20Time) true) false false)))
    (:then_1
      ;[1 1 1] Friction
      (bind _returnvalue (Physics|GetPhysicsLinearVelocity (Variables|Default|GetPlane) "None"))
      (Variables|Default|SetPrev%20Friction _returnvalue)
      (Physics|AddForce (Variables|Default|GetPlane) (* (* (Variables|Default|GetPrev%20Friction) (+ (* (Math|Float|MapRangeClamped (Math|Float|Absolute(Float) (.yaw (CallFunction|GetRotationfromTwoVectors (Variables|Default|GetPrev%20Friction) (Math|Vector|GetForwardVector (Variables|Default|GetPlane))))) 0.0 9e+01 0.0 1.0) (Variables|Parameters|GetAngled%20Friction%20Multiplier)) 1.0 (Math|Float|MapRangeClamped (- (Math|Vector|VectorLength (Variables|Default|GetPrev%20Friction)) (Variables|Parameters|GetMax%20Speed)) 0.0 5e+03 0.0 1.0))) -1.0) "None" true))
    (:then_2
      (Transformation|SetRelativeRotation _plane (Math|Rotator|MakeRotator 0.0 0.0 (.yaw (Variables|/Script/Engine.SceneComponent|GetRelativeRotation _plane))) false false))))

(fn ConstructionScript
  (Variables|Turning|SetCurrent%20Angle (.yaw (Transformation|GetWorldRotation (Variables|Default|GetPlane))))
  (CallFunction|LoadCharacter "Tim"))

(fn LoadCharacter
  (params (Character :type Name))
  (Utilities|FlowControl|Sequence
    (:then_0
      (bind _returnvalue (Utilities|GetDataTableRow "/Game/Data/Character_Data.Character_Data" Character)
        (:then
          (Variables|Parameters|SetAcceleration%20Amount (.Acceleration (Utilities|Struct|BreakCharacter_Struct _returnvalue)))
          (Variables|Parameters|SetReverse%20Amount (.ReverseAcceleration (Utilities|Struct|BreakCharacter_Struct _returnvalue)))
          (Variables|Parameters|SetBrake%20Amount (.Braking (Utilities|Struct|BreakCharacter_Struct _returnvalue)))
          (Variables|Parameters|SetMaxTurn (.MaxTurn (Utilities|Struct|BreakCharacter_Struct _returnvalue)))
          (Variables|Parameters|SetTurn%20Lerp%20Length (.TurnLerpLength (Utilities|Struct|BreakCharacter_Struct _returnvalue)))
          (Variables|Parameters|SetAngled%20Friction%20Multiplier 0.0)
          (Variables|Parameters|SetMax%20Speed (.MaxSpeed (Utilities|Struct|BreakCharacter_Struct _returnvalue))))))
    (:then_1
      (if (Utilities|Name|Equal(Name) Character "Tim")
        (Rendering|Components|Light|SetLightColor (Variables|Default|GetPointLight) "(R=0.658375,G=0.068478,B=0.019382,A=1.000000)" true)
        (Rendering|Components|Light|SetLightColor (Variables|Default|GetPointLight1) "(R=0.658375,G=0.068478,B=0.019382,A=1.000000)" true)
        (else
          (Rendering|Components|Light|SetLightColor (Variables|Default|GetPointLight) "(R=0.000000,G=0.174647,B=0.658375,A=1.000000)" true)
          (Rendering|Components|Light|SetLightColor (Variables|Default|GetPointLight1) "(R=0.000000,G=0.174647,B=0.658375,A=1.000000)" true))))))