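; Car camera actor that eases its scene root toward a requested world location and rotation over timed blends.
; UpdateLocation and UpdateRotation each store a new target, capture the current root transform as the start and reset their own timer.
; Tick advances both timers and linearly interpolates position and rotation independently, using clamped alphas from separate blend lengths.
; The construction script seeds start and target with the root's initial transform.
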(event EventTick
  (params (DeltaSeconds :type Float%20%28single-precision%29))
  (Variables|Default|SetRotation%20Time (+ (Variables|Default|GetRotation%20Time) DeltaSeconds))
  (Variables|Default|SetLocation%20Time (+ (Variables|Default|GetLocation%20Time) DeltaSeconds))
  (Variables|Default|SetRotation%20Alpha (Math|Float|MapRangeClamped (Variables|Default|GetRotation%20Time) 0.0 (Variables|Default|GetLerp%20Rotation%20Length) 0.0 1.0))
  (Variables|Default|SetLocation%20Alpha (Math|Float|MapRangeClamped (Variables|Default|GetLocation%20Time) 0.0 (Variables|Default|GetLerp%20Location%20Length) 0.0 1.0))
  (Transformation|SetWorldRotation (Variables|Default|GetDefaultSceneRoot) (Math|Rotator|Lerp(Rotator) (Variables|Default|GetStart%20Rotation) (Variables|Default|GetDesired%20Rotation) (Variables|Default|GetRotation%20Alpha)) false false)
  (Transformation|SetWorldLocation (Variables|Default|GetDefaultSceneRoot) (Math|Vector|Lerp(Vector) (Variables|Default|GetStart%20Location) (Variables|Default|GetDesired%20Location) (Variables|Default|GetLocation%20Alpha)) false false))

(fn ConstructionScript
  (bind _defaultsceneroot (Variables|Default|GetDefaultSceneRoot))
  (bind _defaultsceneroot_2 (Variables|Default|GetDefaultSceneRoot))
  (bind _returnvalue (Transformation|GetWorldLocation _defaultsceneroot))
  (bind _returnvalue_2 (Transformation|GetWorldRotation _defaultsceneroot_2))
  (Variables|Default|SetDesired%20Location _returnvalue)
  (Variables|Default|SetStart%20Location _returnvalue)
  (Variables|Default|SetDesired%20Rotation _returnvalue_2)
  (Variables|Default|SetStart%20Rotation _returnvalue_2))

(fn UpdateLocation
  (params (Desired%20Location :type Vector))
  (Variables|Default|SetDesired%20Location Desired%20Location)
  (Variables|Default|SetStart%20Location (Transformation|GetWorldLocation (Variables|Default|GetDefaultSceneRoot)))
  (Variables|Default|SetLocation%20Time 0.0))

(fn UpdateRotation
  (params (Desired%20Rotation :type Rotator))
  (Variables|Default|SetDesired%20Rotation Desired%20Rotation)
  (Variables|Default|SetStart%20Rotation (Transformation|GetWorldRotation (Variables|Default|GetDefaultSceneRoot)))
  (Variables|Default|SetRotation%20Time 0.0))