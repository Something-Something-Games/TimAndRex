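; Police car AI controller that chases the TimAndRexCar_BP player car by driving along navmesh paths.
; A looping timer re-runs a synchronous pathfind from the controlled pawn to the target car's location twice a second.
; Tick advances through path points within an acceptance radius, accelerating when facing the current point and otherwise steering PoliceCar_BP1 with strength scaled by yaw error.
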(event Custom|Move%20To
  (params (Destination :type Vector) (TargetActor :type Actor%20Object%20Reference) (AcceptanceRadius :type Float%20%28single-precision%29) (bStopOnOverlap :type Boolean))
  (bind _returnvalue (Pawn|GetControlledPawn))
  (Variables|Default|SetAcceptance%20Radius AcceptanceRadius)
  (Utilities|IsValid TargetActor
    (:Is%20Not%20Valid
      (bind _returnvalue_2 (Class|NavigationSystemV1|FindPathtoLocationSynchronously (Transformation|GetActorLocation _returnvalue) Destination _returnvalue 0))
      (Variables|Default|SetPath%20Points (Variables|/Script/NavigationSystem.NavigationPath|GetPathPoints _returnvalue_2))
      (Variables|Default|SetCurrent%20Point 1))))

(event Custom|Update%20Target
  (bind _returnvalue (Actor|GetActorOfClass "/Game/Blueprints/TimAndRexCar_BP.TimAndRexCar_BP_C"))
  (CallFunction|Moveto (Transformation|GetWorldLocation (Variables|/Game/Blueprints/TimAndRexCar_BP.TimAndRexCar_BP_C|GetBox _returnvalue)) 0 2.5e+02 false))

(event EventBeginPlay
  (Utilities|FlowControl|Delay 0.2)
  (bind _returnvalue (Actor|GetActorOfClass "/Game/Blueprints/TimAndRexCar_BP.TimAndRexCar_BP_C"))
  (CallFunction|Moveto (Transformation|GetWorldLocation (Variables|/Game/Blueprints/TimAndRexCar_BP.TimAndRexCar_BP_C|GetBox _returnvalue)) 0 2.5e+02 false)
  (Utilities|Time|SetTimerbyEvent (delegate Custom|Update%20Target) 0.5 true))

(event EventTick
  (params (DeltaSeconds :type Float%20%28single-precision%29))
  (if (> (Utilities|Array|Length (Variables|Default|GetPath%20Points)) 0)
    (bind _in_radius (CallFunction|CheckifPointinAcceptanceRadius))
    (if _in_radius
      (bind _result (Math|Integer|IncrementInt (Variables|Default|GetCurrent%20Point))
        (:%20%20
          (if (> _result (Utilities|Array|Length (Variables|Default|GetPath%20Points)))
            (Utilities|Array|Clear (Variables|Default|GetPath%20Points))
            (else
              (bind _required_turn (CallFunction|GetRotationtoTarget :!label _label))
              (if (CallFunction|CheckRotationinTolerance _required_turn 1e+01)
                ;[1 1 1] Go to target
                (bind _aspolice_car_bp1 (Utilities|Casting|CastToPoliceCar_BP1 (Pawn|GetControlledPawn)))
                (Default|Accelerate _aspolice_car_bp1 1.0)
                (else
                  ;[1 1 1] Turn to target
                  (bind _turn_left_ (CallFunction|ShouldTurnLeft _required_turn))
                  (if _turn_left_
                    (bind _aspolice_car_bp1_2 (Utilities|Casting|CastToPoliceCar_BP1 (Pawn|GetControlledPawn)))
                    (Default|TurnRight _aspolice_car_bp1_2 (Math|Float|MapRangeUnclamped (Math|Float|Absolute(Float) (.Yaw (Math|Rotator|BreakRotator _required_turn))) 0.0 3.6e+02 -0.45 -1.0))
                    (else
                      (bind _aspolice_car_bp1_3 (Utilities|Casting|CastToPoliceCar_BP1 (Pawn|GetControlledPawn)))
                      (Default|TurnRight _aspolice_car_bp1_3 (Math|Float|MapRangeUnclamped (Math|Float|Absolute(Float) (.Yaw (Math|Rotator|BreakRotator _required_turn))) 0.0 3.6e+02 0.45 1.0))))))))))
      (else
        (goto _label)))))

(fn ConstructionScript)

(fn GetRotationtoTarget
  (bind _path_points (Variables|Default|GetPath%20Points))
  (bind _current_point (Variables|Default|GetCurrent%20Point))
  (bind _output (Utilities|Array|Get(acopy) _path_points _current_point))
  (bind _aspolice_car_bp1 (Utilities|Casting|CastToPoliceCar_BP1 (Pawn|GetControlledPawn)))
  (return (CallFunction|GetRotationfromTwoVectors (Math|Vector|Normalize (- (Math|Vector|MakeVector (.x _output) (.y _output) 0.0) (Math|Vector|MakeVector (.x (Transformation|GetWorldLocation (Variables|/Game/Blueprints/Police/PoliceCar_BP1.PoliceCar_BP1_C|GetBox _aspolice_car_bp1))) (.y (Transformation|GetWorldLocation (Variables|/Game/Blueprints/Police/PoliceCar_BP1.PoliceCar_BP1_C|GetBox _aspolice_car_bp1))) 0.0))) (Math|Vector|GetForwardVector (Variables|/Game/Blueprints/Police/PoliceCar_BP1.PoliceCar_BP1_C|GetBox _aspolice_car_bp1)))))

(fn CheckRotationinTolerance
  (params (Rotation :type Rotator) (Tolerance :type Float%20%28single-precision%29))
  (return (and (and (< (Math|Float|Absolute(Float) (.roll Rotation)) Tolerance) (< (Math|Float|Absolute(Float) (.pitch Rotation)) Tolerance)) (< (Math|Float|Absolute(Float) (.yaw Rotation)) Tolerance))))

(fn CheckifPointinAcceptanceRadius
  (bind _aspolice_car_bp1 (Utilities|Casting|CastToPoliceCar_BP1 (Pawn|GetControlledPawn))
    (:then
      (return (<= (Math|Vector|Distance(Vector) (Transformation|GetWorldLocation (Variables|/Game/Blueprints/Police/PoliceCar_BP1.PoliceCar_BP1_C|GetBox _aspolice_car_bp1)) (Utilities|Array|Get(acopy) (Variables|Default|GetPath%20Points) (Variables|Default|GetCurrent%20Point))) (Variables|Default|GetAcceptance%20Radius))))
    (:CastFailed
      (return false))))

(fn ShouldTurnLeft
  (params (Rotation :type Rotator))
  (bind _returnvalue (Math|Float|Absolute(Float) (.yaw Rotation)))
  (bind _returnvalue_2 (< _returnvalue 1.8e+02))
  (if (< (.yaw Rotation) 0.0)
    (if _returnvalue_2
      _
      (else
        (return false)))
    (elif _returnvalue_2
      (return false)
      (else
        _)))
  (return true))