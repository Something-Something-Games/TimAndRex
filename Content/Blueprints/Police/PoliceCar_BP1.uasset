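; Police car driven as a physics box, with red and blue lights flashing alternately on a looping timer.
; Construction loads handling values from the "Police" row of Character_Data.
; TurnRight, Accelerate, Reverse and Brake events set target yaw or apply forces, with a timeline serving as a speed-based acceleration curve.
; Tick lerps yaw, locks pitch and roll, and applies friction that rises above max speed, with a slip-angle term zeroed on load.
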(event Custom|Reverse
  (params (Amount :type Float%20%28single-precision%29))
  ;[1 1 1] Reverse
  (Physics|AddForce (Variables|Default|GetBox) (* (Math|Vector|GetForwardVector (Variables|Default|GetBox)) (* Amount (Variables|Parameters|GetReverse%20Amount))) "None" true))

(event Custom|Brake
  (params (Amount :type Float%20%28single-precision%29))
  ;[1 1 1] Braking
  (bind _returnvalue (Physics|GetPhysicsLinearVelocity (Variables|Default|GetBox) "None"))
  (Physics|AddForce (Variables|Default|GetBox) (* (* _returnvalue (+ (* (Math|Float|MapRangeClamped (Math|Float|Absolute(Float) (.yaw (CallFunction|GetRotationfromTwoVectors _returnvalue (Math|Vector|GetForwardVector (Variables|Default|GetBox))))) 0.0 9e+01 0.0 1.0) (Variables|Parameters|GetBrake%20Amount)) 1.0)) Amount) "None" true))

(event Custom|Accelerate
  (params (Amount :type Float%20%28single-precision%29))
  ;[1 1 1] Acceleration
  (Variables|Default|SetAcceleration Amount)
  (bind _returnvalue (Physics|GetPhysicsLinearVelocity (Variables|Default|GetBox) "None"))
  (CallFunction|LookupAcceleration (Math|Float|MapRangeClamped (Math|Vector|VectorLength _returnvalue) 0.0 5e+03 0.0 1.0)))

(event Custom|Lookup%20Acceleration
  (params (Lookup%20Value :type Float%20%28single-precision%29))
  ;[1 1 1] Acceleration
  (bind _acceleration (Timeline|Acceleration%20Lookup SetNewTime)
    (:Update
      (CallFunction|ReturnAccelerationLookup _acceleration))))

(event Custom|Turn%20Right
  (params (Amount :type Float%20%28single-precision%29))
  (bind _rotation (Variables|Turning|GetRotation))
  ;[1 1 1] Turning Input
  (Variables|Turning|SetTurn%20Direction Amount)
  (bind _returnvalue (Physics|GetPhysicsLinearVelocity (Variables|Default|GetBox) "None"))
  (bind _output_get (Variables|Turning|SetTurnAngle (* Amount (* (Variables|Parameters|GetMaxTurn) (Math|Float|MapRangeClamped (Math|Float|Absolute(Float) (Math|Vector|VectorLength _returnvalue)) 0.0 1e+03 1.0 1.0)))))
  (Variables|Turning|SetDesired%20Angle (+ _output_get (.yaw _rotation)))
  (Variables|Turning|SetCurrent%20Angle (.yaw _rotation))
  (Variables|Turning|SetCurr%20Turn%20Time 0.0)
  (if (< (Variables|Turning|GetDesired%20Angle) 0.0)
    (Variables|Turning|SetDesired%20Angle (+ (Variables|Turning|GetDesired%20Angle) 3.6e+02))))

(event Custom|Return%20Acceleration%20Lookup
  (params (Acceleration :type Float%20%28single-precision%29))
  ;[1 1 1] Acceleration
  (Physics|AddForce (Variables|Default|GetBox) (* (Math|Vector|GetForwardVector (Variables|Default|GetBox)) (* (* Acceleration (Variables|Default|GetAcceleration)) (Variables|Parameters|GetAcceleration%20Amount))) "None" true))

(event Custom|Flash%20Light
  (Utilities|FlowControl|FlipFlop
    (:A
      (Rendering|Components|Light|SetIntensity (Variables|Default|GetRedLight) 6e+03)
      (Rendering|Components|Light|SetIntensity (Variables|Default|GetBlueLight) 0.0))
    (:B
      (Rendering|Components|Light|SetIntensity (Variables|Default|GetRedLight) 0.0)
      (Rendering|Components|Light|SetIntensity (Variables|Default|GetBlueLight) 6e+03))))

(event EventBeginPlay
  (Utilities|Time|SetTimerbyEvent (delegate Custom|Flash%20Light) 0.5 true))

(event EventTick
  (params (DeltaSeconds :type Float%20%28single-precision%29))
  (Utilities|FlowControl|Sequence
    (:then_1
      ;[1 1 1] Turning
      (if (!= (Variables|Turning|GetCurrent%20Angle) (Variables|Turning|GetDesired%20Angle))
        (Variables|Turning|SetCurr%20Turn%20Time (+ (Variables|Turning|GetCurr%20Turn%20Time) DeltaSeconds))
        (Transformation|SetRelativeRotation (Variables|Default|GetBox) (Math|Rotator|Lerp(Rotator) (Math|Rotator|MakeRotator (.roll (Variables|Turning|GetRotation)) (.pitch (Variables|Turning|GetRotation)) (Variables|Turning|GetCurrent%20Angle)) (Math|Rotator|MakeRotator (.roll (Variables|Turning|GetRotation)) (.pitch (Variables|Turning|GetRotation)) (Variables|Turning|GetDesired%20Angle)) (Variables|Turning|GetCurr%20Turn%20Time) true) false false)
        (Variables|Turning|SetRotation (Math|Rotator|Lerp(Rotator) (Math|Rotator|MakeRotator (.roll (Variables|Turning|GetRotation)) (.pitch (Variables|Turning|GetRotation)) (Variables|Turning|GetCurrent%20Angle)) (Math|Rotator|MakeRotator (.roll (Variables|Turning|GetRotation)) (.pitch (Variables|Turning|GetRotation)) (Variables|Turning|GetDesired%20Angle)) (Variables|Turning|GetCurr%20Turn%20Time) true))))
    (:then_2
      ;[1 1 1] Friction
      (bind _returnvalue (Physics|GetPhysicsLinearVelocity (Variables|Default|GetBox) "None"))
      (Variables|Default|SetPrev%20Friction _returnvalue)
      (Physics|AddForce (Variables|Default|GetBox) (* (* (Variables|Default|GetPrev%20Friction) (+ (* (Math|Float|MapRangeClamped (Math|Float|Absolute(Float) (.yaw (CallFunction|GetRotationfromTwoVectors (Variables|Default|GetPrev%20Friction) (Math|Vector|GetForwardVector (Variables|Default|GetBox))))) 0.0 9e+01 0.0 1.0) (Variables|Parameters|GetAngled%20Friction%20Multiplier)) 1.0 (Math|Float|MapRangeClamped (- (Math|Vector|VectorLength (Variables|Default|GetPrev%20Friction)) (Variables|Parameters|GetMax%20Speed)) 0.0 5e+03 0.0 1.0))) -1.0) "None" true))
    (:then_3
      (Transformation|SetRelativeRotation (Variables|Default|GetBox) (Math|Rotator|MakeRotator 0.0 0.0 (.yaw (Variables|Turning|GetRotation))) false false)
      (Variables|Turning|SetRotation (Math|Rotator|MakeRotator 0.0 0.0 (.yaw (Variables|Turning|GetRotation)))))))

(fn ConstructionScript
  (bind _box (Variables|Default|GetBox))
  (bind _returnvalue (Transformation|GetWorldLocation _box))
  (Variables|Turning|SetCurrent%20Angle (.yaw (Transformation|GetWorldRotation (Variables|Default|GetBox))))
  (Transformation|SetWorldLocation _box (Math|Vector|MakeVector (.x _returnvalue) (.y _returnvalue) 8e+01) false false)
  (CallFunction|LoadCharacter "Police")
  (Variables|Turning|SetRotation (Variables|/Script/Engine.SceneComponent|GetRelativeRotation (Variables|Default|GetBox))))

(fn LoadCharacter
  (params (Character :type Name))
  (Utilities|FlowControl|Sequence
    (:then_0
      (bind _returnvalue (Utilities|GetDataTableRow "/Game/Data/Character_Data.Character_Data" Character)
        (:then
          (Variables|Parameters|SetAcceleration%20Amount (.Acceleration (Utilities|Struct|BreakCharacter_Struct _returnvalue)))
          (Variables|Parameters|SetReverse%20Amount (.ReverseAcceleration (Utilities|Struct|BreakCharacter_Struct _returnvalue)))
          (Variables|Parameters|SetBrake%20Amount (.Braking (Utilities|Struct|BreakCharacter_Struct _returnvalue)))
          (Variables|Parameters|SetMaxTurn (.MaxTurn (Utilities|Struct|BreakCharacter_Struct _returnvalue)))
          (Variables|Parameters|SetTurn%20Lerp%20Length (.TurnLerpLength (Utilities|Struct|BreakCharacter_Struct _returnvalue)))
          (Variables|Parameters|SetAngled%20Friction%20Multiplier 0.0)
          (Variables|Parameters|SetMax%20Speed (.MaxSpeed (Utilities|Struct|BreakCharacter_Struct _returnvalue))))))))