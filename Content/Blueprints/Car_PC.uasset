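; Car_PC is the player controller for driving the Tim and Rex car.
; It forwards accelerate, brake, reverse and turn axis input to the controlled TimAndRexCar_BP pawn.
; The Swap Character action toggles the current character between Tim and Rex, updating the portrait widget created on BeginPlay and having the car load that character.
; A SetCamera event switches the view target to a supplied camera.
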(event Custom|Set%20Camera
  (params (Camera :type Actor%20Object%20Reference))
  (Game|Player|SetViewTargetwithBlend Camera 0.0 "VTBlend_Linear" 0.0 false))

(event EventBeginPlay
  (bind _returnvalue (UserInterface|CreateWidget "/Game/UI/CharacterPortraits_Widget.CharacterPortraits_Widget_C" self))
  (bind _output_get (Variables|Default|SetCharacter%20Portrait _returnvalue))
  (UserInterface|Viewport|AddtoViewport _output_get 0))

(event Input|ActionEvents|InputActionSwapCharacter
  (params (Key :type Key%20Structure :default "None"))
  (:Pressed
    (if (Utilities|Name|Equal(Name) (Variables|Default|GetCurrent%20Character) "Tim")
      (Variables|Default|SetCurrent%20Character "Rex")
      (else
        (Variables|Default|SetCurrent%20Character "Tim")))
    (Default|UpdateCharacter (Variables|Default|GetCharacter%20Portrait) (Variables|Default|GetCurrent%20Character))
    (bind _astim_and_rex_car_bp (Utilities|Casting|CastToTimAndRexCar_BP (Pawn|GetControlledPawn)))
    (Default|LoadCharacter _astim_and_rex_car_bp (Variables|Default|GetCurrent%20Character))))

(event Input|AxisEvents|InputAxisAccelerate
  (params (AxisValue :type Float%20%28single-precision%29))
  (bind _astim_and_rex_car_bp (Utilities|Casting|CastToTimAndRexCar_BP (Pawn|GetControlledPawn)))
  (Default|Accelerate _astim_and_rex_car_bp AxisValue))

(event Input|AxisEvents|InputAxisBrake
  (params (AxisValue :type Float%20%28single-precision%29))
  (bind _astim_and_rex_car_bp (Utilities|Casting|CastToTimAndRexCar_BP (Pawn|GetControlledPawn)))
  (Default|Brake _astim_and_rex_car_bp AxisValue))

(event Input|AxisEvents|InputAxisReverse
  (params (AxisValue :type Float%20%28single-precision%29))
  (bind _astim_and_rex_car_bp (Utilities|Casting|CastToTimAndRexCar_BP (Pawn|GetControlledPawn)))
  (Default|Reverse _astim_and_rex_car_bp AxisValue))

(event Input|AxisEvents|InputAxisTurnRight
  (params (AxisValue :type Float%20%28single-precision%29))
  (bind _astim_and_rex_car_bp (Utilities|Casting|CastToTimAndRexCar_BP (Pawn|GetControlledPawn)))
  (Default|TurnRight _astim_and_rex_car_bp AxisValue))

(fn ConstructionScript)